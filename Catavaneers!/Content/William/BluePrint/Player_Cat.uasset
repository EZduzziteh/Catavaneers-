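; Player cat Blueprint that links the player's inventory to the caravan through input-driven, prototype-style interactions.
; On BeginPlay it finds BP_Caravan_Vi actors and caches the caravan and its inventory.
; Inputs print player stats, hand over wood by overwriting the caravan's amount and zeroing the player's, and toggle caravan part attachment.
; Buying a trap only prints a message, and the N key sets test wood.
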(event EventTick
  (params (DeltaSeconds :type Float%20%28single-precision%29))
  ;[0 0.04334 1] Alejandro drop wood/buy
)

(event EventBeginPlay
  ;[1 0 0] BEGIN
  (bind _outactors (Actor|GetAllActorsOfClass "/Game/Vi/Bluprints/BP_Caravan_Vi.BP_Caravan_Vi_C"))
  (for _array_element _outactors
    (bind _output_get (Variables|Default|SetCaravanRef _array_element))
    (bind _output_get_2 (Variables|Default|SetInventoryReference (Variables|/Game/Vi/Bluprints/BP_Caravan_Vi.BP_Caravan_Vi_C|GetCaravan_inventory _output_get)))
    (Development|PrintString (Utilities|GetDisplayName _output_get_2))))

(event Input|ActionEvents|InputActionAttach/DetachParts
  (params (Key :type Key%20Structure :default "None"))
  (bind _caravanref (Variables|Default|GetCaravanRef))
  ;[1 0 0.1019] Vi attach
  (:Pressed
    (bind _has_part (Default|CheckHasPart _caravanref))
    (if _has_part
      (Default|DetachParts _caravanref)
      (else
        (Default|AttachParts _caravanref)))))

(event Input|ActionEvents|InputActionprintplayer
  (params (Key :type Key%20Structure :default "None"))
  ;[0.06227 0.06198 1] Alejandro Print
  (:Pressed
    (Development|PrintString (Utilities|String|Append (Utilities|String|ToString(Text) (Utilities|Text|MakeLiteralText "Wood = ")) (Utilities|String|ToString(Integer) (Variables|/Script/Catavaneer_2020.Player_inventory|Getwood (Variables|Default|GetBP_player_inventory)))) true true "(R=0.000000,G=0.660000,B=1.000000,A=1.000000)" 1.0)
    (Development|PrintString (Utilities|String|Append (Utilities|String|ToString(Text) (Utilities|Text|MakeLiteralText "GP = ")) (Utilities|String|ToString(Integer) (Variables|/Script/Catavaneer_2020.Player_inventory|GetGP (Variables|Default|GetBP_player_inventory)))) true true "(R=0.000000,G=0.660000,B=1.000000,A=1.000000)" 1.0)
    (Development|PrintString (Utilities|String|Append (Utilities|String|ToString(Text) (Utilities|Text|MakeLiteralText "Trap 1 = ")) (Utilities|String|ToString(Integer) (Variables|/Script/Catavaneer_2020.Player_inventory|GetTrap1 (Variables|Default|GetBP_player_inventory)))) true true "(R=0.000000,G=0.660000,B=1.000000,A=1.000000)" 1.0)
    (Development|PrintString (Utilities|String|Append (Utilities|String|ToString(Text) (Utilities|Text|MakeLiteralText "Trap 2 = ")) (Utilities|String|ToString(Integer) (Variables|/Script/Catavaneer_2020.Player_inventory|GetTrap2 (Variables|Default|GetBP_player_inventory)))) true true "(R=0.000000,G=0.660000,B=1.000000,A=1.000000)" 1.0)
    (Development|PrintString (Utilities|String|Append (Utilities|String|ToString(Text) (Utilities|Text|MakeLiteralText "Score = ")) (Utilities|String|ToString(Integer) (Variables|/Script/Catavaneer_2020.Player_inventory|Getscore (Variables|Default|GetBP_player_inventory)))) true true "(R=0.000000,G=0.660000,B=1.000000,A=1.000000)" 1.0)))

(event Input|ActionEvents|InputActionbuytrap
  (params (Key :type Key%20Structure :default "None"))
  ;[0 0.04334 1] Alejandro drop wood/buy
  (:Pressed
    (Development|PrintString "buy a trap" true true "(R=0.000000,G=0.660000,B=1.000000,A=1.000000)" 1.0)))

(event Input|ActionEvents|InputActiondropwood
  (params (Key :type Key%20Structure :default "None"))
  (bind _inventoryreference (Variables|Default|GetInventoryReference))
  ;[0 0.04334 1] Alejandro drop wood/buy
  (:Pressed
    (Development|PrintString "Give wood to caravan" true true "(R=0.000000,G=0.660000,B=1.000000,A=1.000000)" 1.0)
    (Variables|/Script/Catavaneer_2020.Caravan_inventory|Setwood _inventoryreference (Variables|/Script/Catavaneer_2020.Player_inventory|Getwood (Variables|Default|GetBP_player_inventory)))
    (Development|PrintString (Utilities|String|Append (Utilities|String|ToString(Text) (Utilities|Text|MakeLiteralText "Wood = ")) (Utilities|String|ToString(Integer) (Variables|/Script/Catavaneer_2020.Caravan_inventory|Getwood _inventoryreference))))
    (Variables|/Script/Catavaneer_2020.Player_inventory|Setwood (Variables|Default|GetBP_player_inventory) 0)))

(event Input|KeyboardEvents|N
  (params (Key :type Key%20Structure :default "None"))
  (:Pressed
    (Variables|/Script/Catavaneer_2020.Player_inventory|Setwood (Variables|Default|GetBP_player_inventory) 100)))

(fn ConstructionScript)