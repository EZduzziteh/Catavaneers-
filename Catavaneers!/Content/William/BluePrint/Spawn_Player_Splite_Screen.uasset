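; Actor Blueprint that spawns the local split-screen players when play begins.
; It gathers every PlayerStart, then matches each player index below MaxPlayerCount to a start whose tag equals that number.
; For each match it creates a local player, spawns a Player_Cat at that start, possesses it with that player's controller and records it in the Player array.
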(event EventBeginPlay
  (CallFunction|GetPlayerStartPoint)
  (CallFunction|SpawnPlayer))

(event EventTick
  (params (DeltaSeconds :type Float%20%28single-precision%29)))

(fn ConstructionScript)

(fn GetPlayerStartPoint
  (bind _outactors (Actor|GetAllActorsOfClass "/Script/Engine.PlayerStart"))
  (Variables|Default|Setplayer_Start_Array _outactors))

(fn SpawnPlayer
  (for _index (range 0 (- (Variables|Default|Getmax_Player_Count) 1))
    (Variables|Default|Setindex _index)
    (for _array_element (Variables|Default|Getplayer_Start_Array)
      (if (Utilities|Name|Equal(Name) (Variables|/Script/Engine.PlayerStart|GetPlayerStartTag _array_element) (Utilities|String|StringToName (Utilities|String|ToString(Integer) (Variables|Default|Getindex))))
        (Class|GameplayStatics|CreatePlayer (Variables|Default|Getindex))
        (bind _returnvalue (Game|SpawnActorfromClass "/Game/William/BluePrint/Player_Cat.Player_Cat_C" (Transformation|GetActorTransform _array_element) "AlwaysSpawn" 0 0))
        (Pawn|Possess (Game|GetPlayerController (Variables|Default|Getindex)) _returnvalue)
        (Utilities|Array|AddUnique (Variables|Default|GetPlayer) _returnvalue)))))