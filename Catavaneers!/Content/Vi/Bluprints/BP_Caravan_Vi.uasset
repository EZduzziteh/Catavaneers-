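; Caravan actor that travels between start, stop and end point actors and carries attachable parts.
; BeginPlay teleports it to the start point; Tick eases it to the stop point, then toward the end point once inventory wood reaches the threshold.
; Attach and detach functions snap parts onto Cube sockets matched by object name or restore their start transforms, updating a part count.
; LeaveNode is an unfinished stub.
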(event EventBeginPlay
  ;[1 0 0.171] Vi
  (bind _outactors (Actor|GetAllActorsOfClass "/Game/Vi/Bluprints/BP_Part_Vi.BP_Part_Vi_C"))
  (Variables|Default|SetParts _outactors)
  (Variables|Default|SetSocket%20Names (Transformation|GetAllSocketNames (Variables|Default|GetCube)))
  ;[1 0 0.8715] Josh
  (bind _outactors_2 (Actor|GetAllActorsOfClass "/Game/Josh/StartPoint_Blueprint.StartPoint_Blueprint_C"))
  (bind _array_element (Utilities|Array|ForEachLoopwithBreak _outactors_2)
    (:LoopBody
      (Transformation|SetActorLocationAndRotation (Math|Vector|MakeVector (.X (Math|Vector|BreakVector (Transformation|GetActorLocation _array_element))) (.Y (Math|Vector|BreakVector (Transformation|GetActorLocation _array_element))) (.z (Transformation|GetActorLocation))) (Math|Rotator|CombineRotators (Transformation|GetActorRotation) (Transformation|GetActorRotation _array_element)) false true)
      (Variables|Default|Setarrived_bl false))))

(event Collision|EventActorBeginOverlap
  (params (OtherActor :type Actor%20Object%20Reference)))

(event EventTick
  (params (DeltaSeconds :type Float%20%28single-precision%29))
  ;[1 0 0.9021] Josh Move
  (Math|Integer|CompareInt (Variables|/Script/Catavaneer_2020.Caravan_inventory|Getwood (Variables|Default|GetCaravan_inventory)) 100
    (:>
      (Variables|Default|Setcan_move_bl true :!label _label)
      (bind _outactors (Actor|GetAllActorsOfClass "/Game/Josh/EndPoint_Blueprint.EndPoint_Blueprint_C"))
      (bind _array_element (Utilities|Array|ForEachLoopwithBreak _outactors)
        (:LoopBody
          (Components|MoveComponentTo (Variables|Transformation|GetRootComponent) (Math|Vector|MakeVector (.X (Math|Vector|BreakVector (Transformation|GetActorLocation _array_element))) (.Y (Math|Vector|BreakVector (Transformation|GetActorLocation _array_element))) (.z (Transformation|GetActorLocation))) (Math|Rotator|CombineRotators (Transformation|GetActorRotation) (Transformation|GetActorRotation _array_element)) true false (Variables|Default|Getmove_time) false)
          (Development|PrintString "back to map"))))
    (:==
      (goto _label))
    (:<
      (Variables|Default|Setcan_move_bl false)
      (if (not (Variables|Default|Getarrived_bl))
        (bind _outactors_2 (Actor|GetAllActorsOfClass "/Game/Josh/StopPoint_Blueprint.StopPoint_Blueprint_C"))
        (bind _array_element_2 (Utilities|Array|ForEachLoopwithBreak _outactors_2)
          (:LoopBody
            (Components|MoveComponentTo (Variables|Transformation|GetRootComponent) (Math|Vector|MakeVector (.X (Math|Vector|BreakVector (Transformation|GetActorLocation _array_element_2))) (.Y (Math|Vector|BreakVector (Transformation|GetActorLocation _array_element_2))) (.z (Transformation|GetActorLocation))) (Math|Rotator|CombineRotators (Transformation|GetActorRotation) (Transformation|GetActorRotation _array_element_2)) true false (Variables|Default|Getmove_time) true)
            (Variables|Default|Setarrived_bl true)))))))

(fn ConstructionScript)

(fn CheckHasPart
  (return (> (Variables|Default|GetPart%20Count) 0)))

(fn AttachParts
  ;[1 1 1] VI
  (for _array_element (Variables|Default|GetParts)
    (for _array_element_2 (Variables|Default|GetSocket%20Names)
      (if (Utilities|String|Contains (Utilities|GetObjectName _array_element) (Utilities|String|ToString(Name) _array_element_2))
        (Transformation|AttachComponentToComponent (Variables|/Script/Engine.Actor|GetRootComponent _array_element) (Variables|Default|GetCube) _array_element_2 "SnapToTarget" "KeepRelative" "KeepRelative" true)
        (bind _result (Math|Integer|IncrementInt (Variables|Default|GetPart%20Count))
          (:%20%20
            (Variables|Default|SetPart%20Count _result)
            (Variables|/Game/Vi/Bluprints/BP_Part_Vi.BP_Part_Vi_C|SetHas%20Parent _array_element true)))))))

(fn DetachParts
  (for _array_element (Variables|Default|GetParts)
    (Transformation|DetachFromComponent (Variables|/Script/Engine.Actor|GetRootComponent _array_element) "KeepRelative" "KeepRelative" "KeepRelative" true)
    (Transformation|SetActorTransform _array_element (Variables|/Game/Vi/Bluprints/BP_Part_Vi.BP_Part_Vi_C|GetStart%20Transform _array_element))
    (bind _result (Math|Integer|DecrementInt (Variables|Default|GetPart%20Count))
      (:%20%20
        (Variables|Default|SetPart%20Count _result)))))

(fn LeaveNode
  ;[0.8984 0 1] Josh
  (bind _outactors (Actor|GetAllActorsOfClass "/Script/Engine.TriggerBox"))
  (bind _array_element (Utilities|Array|ForEachLoopwithBreak _outactors)))