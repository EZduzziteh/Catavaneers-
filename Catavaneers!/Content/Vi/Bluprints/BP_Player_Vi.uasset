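; Player Blueprint that handles camera look input and lets the player attach or detach parts on the caravan.
; BeginPlay caches the BP_Caravan_Vi actor found in the level through GetActorOfClass.
; The Attach/Detach Parts action toggles on press, detaching if the caravan reports it has a part and attaching otherwise.
; LookUp and LookSideways axes feed controller pitch and yaw directly.
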(event EventBeginPlay
  (bind _returnvalue (Actor|GetActorOfClass "/Game/Vi/Bluprints/BP_Caravan_Vi.BP_Caravan_Vi_C"))
  (Variables|Default|SetCaravan _returnvalue))

(event Collision|EventActorBeginOverlap
  (params (OtherActor :type Actor%20Object%20Reference)))

(event EventTick
  (params (DeltaSeconds :type Float%20%28single-precision%29)))

(event Input|ActionEvents|InputActionAttach/DetachParts
  (params (Key :type Key%20Structure :default "None"))
  (bind _caravan (Variables|Default|GetCaravan))
  (:Pressed
    (bind _has_part (Default|CheckHasPart _caravan))
    (if _has_part
      (Default|DetachParts _caravan)
      (else
        (Default|AttachParts _caravan)))))

(event Input|AxisEvents|InputAxisLookUp
  (params (AxisValue :type Float%20%28single-precision%29))
  (Pawn|Input|AddControllerPitchInput AxisValue))

(event Input|AxisEvents|InputAxisLookSideways
  (params (AxisValue :type Float%20%28single-precision%29))
  (Pawn|Input|AddControllerYawInput AxisValue))

(fn ConstructionScript)