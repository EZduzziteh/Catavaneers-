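; BP_player is the player Blueprint, handling debug readouts and wood hand-off between its BPPlayerInventory and a caravan's inventory.
; BeginPlay caches the CaravanInventory of BP_Caravan_Vi actors, keeping the last one found.
; The drop wood input overwrites the caravan's Wood with the player's, without adding or checking proximity, then zeroes the player's.
; Another input prints resources, traps and score; buy trap only prints a message.
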(event EventBeginPlay
  (bind _outactors (Actor|GetAllActorsOfClass "/Game/Vi/Bluprints/BP_Caravan_Vi.BP_Caravan_Vi_C"))
  (for _array_element _outactors
    (bind _output_get (Variables|Default|SetInventoryReference (Variables|/Game/Vi/Bluprints/BP_Caravan_Vi.BP_Caravan_Vi_C|GetCaravan_inventory _array_element)))
    (Development|PrintString (Utilities|GetDisplayName _output_get))))

(event Collision|EventActorBeginOverlap
  (params (OtherActor :type Actor%20Object%20Reference)))

(event Input|ActionEvents|InputActionprintplayer
  (params (Key :type Key%20Structure :default "None"))
  (:Pressed
    (Development|PrintString (Utilities|String|Append (Utilities|String|ToString(Text) (Utilities|Text|MakeLiteralText "Wood = ")) (Utilities|String|ToString(Integer) (Variables|/Script/Catavaneer_2020.Player_inventory|Getwood (Variables|Default|GetBP_player_inventory)))) true true "(R=0.000000,G=0.660000,B=1.000000,A=1.000000)" 1.0)
    (Development|PrintString (Utilities|String|Append (Utilities|String|ToString(Text) (Utilities|Text|MakeLiteralText "GP = ")) (Utilities|String|ToString(Integer) (Variables|/Script/Catavaneer_2020.Player_inventory|GetGP (Variables|Default|GetBP_player_inventory)))) true true "(R=0.000000,G=0.660000,B=1.000000,A=1.000000)" 1.0)
    (Development|PrintString (Utilities|String|Append (Utilities|String|ToString(Text) (Utilities|Text|MakeLiteralText "Trap 1 = ")) (Utilities|String|ToString(Integer) (Variables|/Script/Catavaneer_2020.Player_inventory|GetTrap1 (Variables|Default|GetBP_player_inventory)))) true true "(R=0.000000,G=0.660000,B=1.000000,A=1.000000)" 1.0)
    (Development|PrintString (Utilities|String|Append (Utilities|String|ToString(Text) (Utilities|Text|MakeLiteralText "Trap 2 = ")) (Utilities|String|ToString(Integer) (Variables|/Script/Catavaneer_2020.Player_inventory|GetTrap2 (Variables|Default|GetBP_player_inventory)))) true true "(R=0.000000,G=0.660000,B=1.000000,A=1.000000)" 1.0)
    (Development|PrintString (Utilities|String|Append (Utilities|String|ToString(Text) (Utilities|Text|MakeLiteralText "Score = ")) (Utilities|String|ToString(Integer) (Variables|/Script/Catavaneer_2020.Player_inventory|Getscore (Variables|Default|GetBP_player_inventory)))) true true "(R=0.000000,G=0.660000,B=1.000000,A=1.000000)" 1.0)))

(event Input|ActionEvents|InputActionbuytrap
  (params (Key :type Key%20Structure :default "None"))
  (:Pressed
    (Development|PrintString "buy a trap" true true "(R=0.000000,G=0.660000,B=1.000000,A=1.000000)" 1.0)))

(event Input|ActionEvents|InputActiondropwood
  (params (Key :type Key%20Structure :default "None"))
  (bind _inventoryreference (Variables|Default|GetInventoryReference))
  (:Pressed
    (Development|PrintString "Give wood to caravan" true true "(R=0.000000,G=0.660000,B=1.000000,A=1.000000)" 1.0)
    (Variables|/Script/Catavaneer_2020.Caravan_inventory|Setwood _inventoryreference (Variables|/Script/Catavaneer_2020.Player_inventory|Getwood (Variables|Default|GetBP_player_inventory)))
    (Development|PrintString (Utilities|String|Append (Utilities|String|ToString(Text) (Utilities|Text|MakeLiteralText "Wood = ")) (Utilities|String|ToString(Integer) (Variables|/Script/Catavaneer_2020.Caravan_inventory|Getwood _inventoryreference))))
    (Variables|/Script/Catavaneer_2020.Player_inventory|Setwood (Variables|Default|GetBP_player_inventory) 0)))

(fn ConstructionScript)