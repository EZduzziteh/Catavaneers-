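; BP_Notice is a clickable notice board job offering a gold reward for a trip between two points.
; On BeginPlay it rolls a distance in nodes, derives gold from it plus random variance, and picks a start point ID from fixed values.
; SelectEndPoint picks an end point ID, calling itself again if it matches the start.
; Clicking passes gold and distance to the NoticeBoard_Pawn's widget and registers itself as that pawn's selected notice.
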(event Custom|Select%20End%20Point
  (switch int (Math|Random|RandomInteger 6)
    (:0
      (Variables|Default|SetEndPoint 12))
    (:1
      (Variables|Default|SetEndPoint 21))
    (:2
      (Variables|Default|SetEndPoint 6))
    (:3
      (Variables|Default|SetEndPoint 10))
    (:4
      (Variables|Default|SetEndPoint 16))
    (:5
      (Variables|Default|SetEndPoint 0)))
  (if (== (Variables|Default|GetStartPoint) (Variables|Default|GetEndPoint))
    (CallFunction|SelectEndPoint)))

(event EventBeginPlay
  (bind _returnvalue (Actor|GetActorOfClass "/Game/Sasha/Menu/NoticeBoard/NoticeBoard_Pawn.NoticeBoard_Pawn_C"))
  (Variables|Default|Setpawnref _returnvalue)
  (bind _output_get (Variables|Default|SetDistance%28nodes%29 (+ 7 (Math|Random|RandomInteger 8))))
  (Variables|Default|SetReward%28Gold%29 (+ (* _output_get (+ (Math|Random|RandomInteger 20) 35)) (Math|Random|RandomInteger 300)))
  (switch int (Math|Random|RandomInteger 6)
    (:Default
      (Variables|Default|SetStartPoint 0 :!label _label))
    (:0
      (Variables|Default|SetStartPoint 12))
    (:1
      (goto _label))
    (:2
      (Variables|Default|SetStartPoint 6))
    (:3
      (Variables|Default|SetStartPoint 21))
    (:4
      (Variables|Default|SetStartPoint 16))
    (:5
      (Variables|Default|SetStartPoint 12)))
  (CallFunction|SelectEndPoint))

(event Collision|EventActorBeginOverlap
  (params (OtherActor :type Actor%20Object%20Reference)))

(event EventTick
  (params (DeltaSeconds :type Float%20%28single-precision%29)))

(event MouseInput|EventActorOnClicked
  (params (ButtonPressed :type Key%20Structure))
  (bind _pawnref (Variables|Default|Getpawnref))
  (bind _widgetref (Variables|/Game/Sasha/Menu/NoticeBoard/NoticeBoard_Pawn.NoticeBoard_Pawn_C|Getwidgetref _pawnref))
  (Variables|/Game/Sasha/Menu/NoticeBoard/NoticeBoard_Hud.NoticeBoard_Hud_C|Setgold _widgetref (Variables|Default|GetReward%28Gold%29))
  (Variables|/Game/Sasha/Menu/NoticeBoard/NoticeBoard_Hud.NoticeBoard_Hud_C|Setdistance _widgetref (Variables|Default|GetDistance%28nodes%29))
  (Variables|/Game/Sasha/Menu/NoticeBoard/NoticeBoard_Pawn.NoticeBoard_Pawn_C|SetNoticeRef _pawnref self))

(fn ConstructionScript)