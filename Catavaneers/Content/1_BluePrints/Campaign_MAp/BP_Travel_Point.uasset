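; Clickable campaign map node that moves the Map_Pawn to itself, spending fuel unless debug infinite fuel bypasses the check.
; Clicking its visible sphere, or a sphere hit, updates the pawn's node and HUD, then a timeline lerps the pawn's location.
; On arrival it opens the victory level at the destination or refreshes point visibility and optionally saves and loads its level, gated by the pawn's IsLoaded flag.
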(event OnComponentHit(Sphere)
  (params (HitComponent :type Primitive%20Component%20Object%20Reference) (OtherActor :type Actor%20Object%20Reference) (OtherComp :type Primitive%20Component%20Object%20Reference) (NormalImpulse :type Vector :default "0, 0, 0") (Hit :type Hit%20Result%20Structure%20%28by%20ref%29))
  ;[1 1 1] Move Triggers
  (CallFunction|MovetoPoint))

(event Custom|MoveToPoint
  (bind _pawnref (Variables|Default|GetPawnRef))
  (bind _pawnref_2 (Variables|Default|GetPawnRef))
  (bind _hudref (Variables|/Game/1_BluePrints/Campaign_MAp/Map_Pawn.Map_Pawn_C|Gethudref _pawnref))
  ;[1 1 1] MoveToPoint
  ;;[1 0.02754 0] Check if Movement Allowed
  (if (Variables|/Game/1_BluePrints/Campaign_MAp/Map_Pawn.Map_Pawn_C|GetDebug_InfiniteFuel _pawnref_2)
    (if (not (Variables|/Game/1_BluePrints/Campaign_MAp/Map_Pawn.Map_Pawn_C|GetMoving _pawnref_2)) :!label _label
      ;;[0.401 0.03757 0.3554] Update Current node on map pawn
      (Variables|/Game/1_BluePrints/Campaign_MAp/Map_Pawn.Map_Pawn_C|Setnoderef _pawnref_2 self)
      (Variables|/Game/1_BluePrints/Campaign_MAp/Map_Pawn.Map_Pawn_C|SetCurrentNodeIndex (Variables|Default|GetPawnRef) (Variables|Default|GetTravelPointIndex))
      ;;[1 0.02728 0.7287] Update Fuel Level
      (Math|Integer|DecrementInt (Variables|/Game/1_BluePrints/Campaign_MAp/Map_Pawn.Map_Pawn_C|GetFuel _pawnref)
        (:%20%20
          (bind _result (Math|Integer|DecrementInt (Variables|/Game/1_BluePrints/Campaign_MAp/Map_Hud.Map_Hud_C|GetFuel%20Level _hudref))
            (:%20%20
              (Variables|/Game/1_BluePrints/Campaign_MAp/Map_Hud.Map_Hud_C|SetFuel%20Level _hudref _result)
              ;;[0.3991 1 0.436] Update Hud
              (Variables|/Game/1_BluePrints/Campaign_MAp/Map_Hud.Map_Hud_C|SetNameToDraw (Variables|/Game/1_BluePrints/Campaign_MAp/Map_Pawn.Map_Pawn_C|Gethudref (Variables|Default|GetPawnRef)) (Variables|Default|GetLocationName))
              (CallFunction|MovePawn))))))
    (elif (> (Variables|/Game/1_BluePrints/Campaign_MAp/Map_Pawn.Map_Pawn_C|GetFuel _pawnref_2) 0)
      (goto _label))))

(event Custom|ToggleInrange
  (params (isactive :type Boolean))
  ;[1 1 1] togglevisible
  (Rendering|SetVisibility (Variables|Default|GetSphere) isactive false)
  (Rendering|SetVisibility (Variables|Default|GetIcon1) isactive false)
  (Rendering|SetVisibility (Variables|Default|GetIcon2) isactive false)
  (Rendering|SetVisibility (Variables|Default|GetIcon3) isactive false))

(event Custom|Try%20Load%20Level
  (bind _pawnref (Variables|Default|GetPawnRef))
  ;[1 1 1] Try Load Level
  (if (Variables|/Game/1_BluePrints/Campaign_MAp/Map_Pawn.Map_Pawn_C|GetIsLoaded _pawnref)
    (Default|SaveInfo (Variables|Default|GetPawnRef))
    (Game|OpenLevel(byName) (Variables|Default|GetLevelToLoad))
    (else
      (Variables|/Game/1_BluePrints/Campaign_MAp/Map_Pawn.Map_Pawn_C|SetIsLoaded _pawnref true))))

(event Custom|Move%20Pawn
  (bind _pawnref (Variables|Default|GetPawnRef))
  (bind _pawnref_2 (Variables|Default|GetPawnRef))
  ;[1 1 1] Move Pawn
  (Variables|/Game/1_BluePrints/Campaign_MAp/Map_Pawn.Map_Pawn_C|SetMoving (Variables|Default|GetPawnRef) true)
  (bind _output_get (Variables|Default|SetStartpos (Transformation|GetActorTransform (Variables|Default|GetPawnRef))))
  (bind _float (Timeline|Timeline_0 PlayFromStart)
    (:Update
      (Transformation|SetActorTransform (Variables|Default|GetPawnRef) (Math|Transform|MakeTransform (Math|Vector|MakeVector (.X (Math|Vector|BreakVector (.Location (Math|Transform|BreakTransform (Math|Transform|Lerp(Transform) _output_get (Transformation|GetActorTransform) _float))))) (.Y (Math|Vector|BreakVector (.Location (Math|Transform|BreakTransform (Math|Transform|Lerp(Transform) _output_get (Transformation|GetActorTransform) _float))))) (.Z (Math|Vector|BreakVector (.Location (Math|Transform|BreakTransform (Math|Transform|Lerp(Transform) _output_get (Transformation|GetActorTransform) _float)))))) (.rotation (Variables|Default|GetStartpos)))))
    (:Finished
      (Variables|/Game/1_BluePrints/Campaign_MAp/Map_Pawn.Map_Pawn_C|SetMoving _pawnref_2 false)
      (if (and (== (Variables|/Game/1_BluePrints/Campaign_MAp/Map_Pawn.Map_Pawn_C|GetDestinationNodeIndex _pawnref) (Variables|Default|GetTravelPointIndex)) (Variables|/Game/1_BluePrints/Campaign_MAp/Map_Pawn.Map_Pawn_C|Getisloaded _pawnref))
        (Game|OpenLevel(byName) "Temp_Victory")
        (else
          (Default|UpdateTravelPointVis _pawnref_2)
          (if (Variables|Default|GetLoadLevel)
            (CallFunction|TryLoadLevel)))))))

(event EventBeginPlay
  ;[1 1 1] BegiPlay
  ;;[1 1 1] Get Reference to Map Pawn
  (bind _outactors (Actor|GetAllActorsOfClass "/Game/1_BluePrints/Campaign_MAp/Map_Pawn.Map_Pawn_C"))
  (for _array_element _outactors
    (Variables|Default|SetPawnRef _array_element)))

(event MouseInput|EventActorOnClicked
  (params (ButtonPressed :type Key%20Structure :default "None"))
  ;[1 1 1] Move Triggers
  (if (Rendering|IsVisible (Variables|Default|GetSphere))
    (Audio|PlaySoundatLocation (Variables|Default|GetSoundOnClick) "0, 0, 0" "0, 0, 0" 1.0 1.0 0.0 0 0 0)
    (CallFunction|MovetoPoint)))

(fn ConstructionScript)