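; BP_MenuOption is a clickable 3D main-menu option that quits the game, loads a level or rotates the menu pawn.
; It displays its text and swaps the cone's material on cursor hover.
; A click plays a sound and, after a delay, branches on its flags.
; Level loading first saves a new SG_Campaign with the Ironcat flag; otherwise a timeline turns Menu_Pawn toward the option's yaw-offset rotation.
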(event EventBeginPlay
  (Rendering|Components|TextRender|SetText (Variables|Default|GetTextRender) (Variables|Default|GetText))
  (bind _returnvalue (Actor|GetActorOfClass "/Game/1_BluePrints/Menu/Main/Menu_Pawn.Menu_Pawn_C"))
  (Variables|Default|SetPawnRef _returnvalue))

(event Collision|EventActorBeginOverlap
  (params (OtherActor :type Actor%20Object%20Reference)))

(event EventTick
  (params (DeltaSeconds :type Float%20%28single-precision%29)))

(event MouseInput|EventActorBeginCursorOver
  (Rendering|Material|SetMaterial (Variables|Default|GetCone) 0 (Variables|Default|GetScrolledMaterial)))

(event MouseInput|EventActorEndCursorOver
  (Rendering|Material|SetMaterial (Variables|Default|GetCone) 0 (Variables|Default|GetDefaultMaterial)))

(event MouseInput|EventActorOnClicked
  (params (ButtonPressed :type Key%20Structure :default "None"))
  (Audio|PlaySoundatLocation (Variables|Default|GetSoundtoPlay) "0, 0, 0" "0, 0, 0" 1.0 1.0 0.0 0 0 0)
  (Utilities|FlowControl|Delay (Variables|Default|GetDelayTimer))
  (if (Variables|Default|GetQuitGame)
    (Game|QuitGame 0 "Quit" false)
    (elif (Variables|Default|GetLoadLevel)
      (bind _returnvalue (SaveGame|CreateSaveGameObject "/Game/1_BluePrints/SaveGames/SG_Campaign.SG_Campaign_C"))
      (Variables|/Game/1_BluePrints/SaveGames/SG_Campaign.SG_Campaign_C|SetIroncat_Enabled _returnvalue (Variables|Default|GetEnableIroncat))
      (|AsyncSaveGametoSlot _returnvalue "Slot1"
        (:Completed
          (Game|OpenLevel(byName) (Variables|Default|GetLevelToLoad))))
      (else
        (Variables|Default|Setendingrotation_0 (Math|Rotator|CombineRotators (Transformation|GetActorRotation) (Math|Rotator|MakeRotator 0.0 0.0 (Variables|Default|Getrotateamount))))
        (bind _newtrack_0 (Timeline|Timeline_0 PlayFromStart)
          (:Update
            (Transformation|SetActorRotation (Variables|Default|GetPawnRef) (Math|Rotator|Lerp(Rotator) (Transformation|GetActorRotation (Variables|Default|GetPawnRef)) (Variables|Default|Getendingrotation_0) _newtrack_0 true))))))))

(fn ConstructionScript)