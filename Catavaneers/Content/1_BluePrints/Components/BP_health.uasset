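; Health component that tracks its owning actor's health and destroys that actor when health reaches zero.
; TakeDamage subtracts damage with a floor of zero, then fires either the OnDeath or OnHealthChanged event dispatcher.
; The component binds to its own dispatchers on BeginPlay, printing a debug line for each hit and a death message before destroying the owner.
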(event Custom|OnHealthChanged
  (params (Damage%20Taken :type Float%20%28single-precision%29) (Current%20Health :type Float%20%28single-precision%29))
  (CallFunction|PrintDebug Damage%20Taken Current%20Health))

(event Custom|OnDeath
  (CallFunction|Death)
  (Actor|DestroyActor (Components|GetOwner)))

(event EventBeginPlay
  (Variables|Default|SetCurrent%20Health (Variables|Default|GetMax%20Health))
  (EventDispatchers|BindEventtoOnHealthChangedEventDispatcher (delegate Custom|OnHealthChanged))
  (EventDispatchers|BindEventtoOnDeathEventDispatcher (delegate Custom|OnDeath)))

(event EventTick
  (params (DeltaSeconds :type Float%20%28single-precision%29)))

(fn TakeDamage
  (params (Damage :type Float%20%28single-precision%29))
  (bind _output_get (Variables|Default|SetCurrent%20Health (Math|Float|Max(Float) (- (Variables|Default|GetCurrent%20Health) Damage) 0.0)))
  (if (== _output_get 0.0)
    (Default|CallOnDeathEventDispatcher)
    (else
      (Default|CallOnHealthChangedEventDispatcher Damage (Variables|Default|GetCurrent%20Health)))))

(fn Death
  (Development|PrintString "You're Dead!!!"))

(fn PrintDebug
  (params (Damage%20Taken :type Float%20%28single-precision%29) (Current%20Health :type Float%20%28single-precision%29))
  (Development|PrintString (Utilities|String|Append (Utilities|String|Append (Utilities|String|Append (Utilities|String|Append (Utilities|GetDisplayName (Components|GetOwner)) " took ") (Utilities|String|ToString(Float) Damage%20Taken)) ", Cureent health = ") (Utilities|String|ToString(Float) Current%20Health))))